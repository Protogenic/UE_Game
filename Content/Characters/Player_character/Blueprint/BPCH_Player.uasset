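; Player character Blueprint that handles camera look, movement and drawing or sheathing a sword.
; Axis inputs move the character relative to control yaw and turn the view, while Tick clamps control pitch to a fixed range.
; The Combat mode action alternates via FlipFlop, playing SM_Sheath, snapping DefaultSword between WeaponOn and WeaponOff on timed delays, then setting CombatMode.
; A DoOnce blocks repeat presses until each swap finishes.
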(event EventBeginPlay)

(event Collision|EventActorBeginOverlap
  (params (OtherActor :type Actor%20Object%20Reference)))

(event EventTick
  (params (DeltaSeconds :type Float%20%28single-precision%29))
  (bind _returnvalue (Pawn|GetControlRotation :!class /Script/Engine.Pawn))
  (Pawn|SetControlRotation (Game|GetPlayerController 0) (Math|Rotator|MakeRotator (.roll _returnvalue) (Math|Float|ClampAngle (.pitch _returnvalue) -45.0 45.0) (.yaw _returnvalue))))

(event Input|ActionEvents|InputActionCombatmode
  (params (Key :type Key%20Structure :default "None"))
  (bind _default_sword (Variables|Default|GetDefault_Sword))
  (:Pressed
    (Utilities|FlowControl|DoOnce false :!label _label
      (:Completed
        (Utilities|FlowControl|FlipFlop
          (:A
            (Animation|PlayAnimMontage "/Game/Characters/Player_character/Animation/Locomotion/Combat/SM_Sheath.SM_Sheath" 1.0 "None")
            (Utilities|FlowControl|Delay 0.85)
            (Transformation|AttachComponentToComponent _default_sword (Variables|Default|GetWeaponOn) "None" "SnapToTarget" "SnapToTarget" "KeepRelative" true)
            (Utilities|FlowControl|Delay 0.55)
            (Variables|Default|SetCombat%20mode true)
            (goto _label Reset))
          (:B
            (Animation|PlayAnimMontage "/Game/Characters/Player_character/Animation/Locomotion/Combat/SM_Sheath.SM_Sheath" 1.0 "None")
            (Utilities|FlowControl|Delay 0.85)
            (Transformation|AttachComponentToComponent _default_sword (Variables|Default|GetWeaponOff) "None" "SnapToTarget" "SnapToTarget" "KeepRelative" true)
            (Utilities|FlowControl|Delay 0.55)
            (Variables|Default|SetCombat%20mode false)
            (goto _label Reset)))))))

(event Input|AxisEvents|InputAxisLookUp
  (params (AxisValue :type Float%20%28single-precision%29))
  (Pawn|Input|AddControllerPitchInput AxisValue))

(event Input|AxisEvents|InputAxisLookRight
  (params (AxisValue :type Float%20%28single-precision%29))
  (Pawn|Input|AddControllerYawInput AxisValue))

(event Input|AxisEvents|InputAxisMoveForward
  (params (AxisValue :type Float%20%28single-precision%29))
  (Pawn|Input|AddMovementInput (Math|Vector|GetForwardVector (Math|Rotator|MakeRotator 0.0 0.0 (.yaw (Pawn|GetControlRotation :!class /Script/Engine.Pawn)))) AxisValue false))

(event Input|AxisEvents|InputAxisMoveRight
  (params (AxisValue :type Float%20%28single-precision%29))
  (Pawn|Input|AddMovementInput (Math|Vector|GetRightVector (Math|Rotator|MakeRotator 0.0 0.0 (.yaw (Pawn|GetControlRotation :!class /Script/Engine.Pawn)))) AxisValue false))

(fn ConstructionScript)